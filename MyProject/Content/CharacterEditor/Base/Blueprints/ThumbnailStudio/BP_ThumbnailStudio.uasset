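; Editor studio actor that renders thumbnail textures for character-customization apparel and hairstyle data assets (CDAs).
; Construction fills a name-to-mesh map from the asset registry by class and anatomy, unless manually edited, and dresses a grey-material basebody from the anatomy profiles table.
; CaptureThumbnailsToContentBrowser swaps in each mesh, captures it via SceneCapture and saves a static texture.
; BeginPlay shows a studio widget fed by the render target.
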(event `self.ReceiveBeginPlay`
  (bind _returnvalue (`GameplayStatics.GetPlayerController` 0))
  (bind _returnvalue_2 (`|CreateWidget` "/Game/CharacterEditor/Base/Widgets/WBP_CDA_ThumbnailStudio.WBP_CDA_ThumbnailStudio_C"))
  (`UserWidget.AddToViewport` _returnvalue_2 0)
  (bind _returnvalue_3 (`|GenericCreateObject` "/Script/Engine.Texture2D" self))
  (`KismetRenderingLibrary.ConvertRenderTargetToTexture2DEditorOnly` (`self.TextureTarget`) _returnvalue_3)
  (`/Game/CharacterEditor/Base/Widgets/WBP_CDA_ThumbnailStudio.Initialize` _returnvalue_2 _returnvalue_3)
  (set `PlayerController.bShowMouseCursor` true _returnvalue)
  (`WidgetBlueprintLibrary.SetInputMode_GameAndUIEx` _returnvalue null))

(fn `CaptureScene`
  (`SceneCaptureComponent2D.CaptureScene` (`self.CaptureComponent2D`)))

(fn `CaptureThumbnailsToContentBrowser`
  (bind _keys (`BlueprintMapLibrary.Map_Keys` (`self.SelectedCDAs`)))
  (for _array_element _keys
    (`SkinnedMeshComponent.SetSkinnedAssetAndUpdate` (`SkeletalMeshActor.SkeletalMeshComponent` (`self.ThumbnailMesh`)) (`BlueprintMapLibrary.Map_Find` (`self.SelectedCDAs`) _array_element) true)
    (`SceneCaptureComponent2D.CaptureScene` (`self.CaptureComponent2D`))
    (bind _returnvalue (`KismetRenderingLibrary.RenderTargetCreateStaticTexture2DEditorOnly` (`SceneCaptureComponent2D.TextureTarget` (`self.CaptureComponent2D`)) _array_element "TC_Default" "TMGS_NoMipmaps"))
    (set `Texture.SRGB` true _returnvalue)
    (set `Texture.CompressionNoAlpha` true _returnvalue)
    (set `Texture.DeferCompression` true _returnvalue)))

(fn `PreloadAllDataAssets`
  (`/Game/CharacterEditor/Base/Blueprints/Libraries/CharacterEditorFunctionLibrary.GetCDA_FromAssetRegistry` "/Game/CharacterEditor/Base/Blueprints/DataAssets/BP_CustomizationDataAsset.BP_CustomizationDataAsset_C")
  (`/Game/CharacterEditor/Base/Blueprints/Libraries/CharacterEditorFunctionLibrary.GetCDA_FromAssetRegistry` "/Game/CharacterEditor/Base/Blueprints/DataAssets/BP_CustomizationDataAsset.BP_CustomizationDataAsset_C" "NewEnumerator0"))

(fn `SetAnatomy`
  (params (Anatomy :type "/Game/CharacterEditor/Base/Enumerations/EAnatomy Enum" :default "NewEnumerator2"))
  (set `self.Anatomy` Anatomy)
  (`self.UpdateGenderVisuals`))

(fn `SetSkeletalMesh`
  (params (NewMesh :type "SkeletalMesh Object Reference"))
  (`SkinnedMeshComponent.SetSkinnedAssetAndUpdate` (`SkeletalMeshActor.SkeletalMeshComponent` (`self.ThumbnailMesh`)) NewMesh true))

(fn `UpdateGenderVisuals`
  (bind _skeletalmeshcomponent (`SkeletalMeshActor.SkeletalMeshComponent` (`self.BasebodyHeadMesh`)))
  (bind _skeletalmeshcomponent_2 (`SkeletalMeshActor.SkeletalMeshComponent` (`self.BasebodyBodyMesh`)))
  (`/Engine/EditorBlueprintResources/StandardMacros.IsValid` (`self.BasebodyBodyMesh`)
    (:`Is Valid`
      (bind _returnvalue (`|GetDataTableRow` "/Game/CharacterEditor/Base/DataTables/DT_AnatomyProfiles.DT_AnatomyProfiles" (`KismetStringLibrary.Conv_StringToName` (`KismetStringLibrary.Replace` (`|GetEnumeratorNameAsString` (`self.Anatomy`)) " ")))
        (:`then`
          (bind ((`BodyMesh_2_5C611F83477EB55EB5235C9B377961CF` _bodymesh) (`HeadMesh_4_C414A762406A620AAA146CB14EF83B87` _headmesh) (`AnimInstanceClass_8_09BC80C1476B7539F7DA9B8EB0589479` _animinstanceclass)) (break `/Game/CharacterEditor/Base/Structures/FAnatomyProfile` _returnvalue))
          (`SkeletalMeshComponent.SetAnimInstanceClass` (`SkeletalMeshActor.SkeletalMeshComponent` (`self.BasebodyBodyMesh`)) _animinstanceclass)
          (`SkeletalMeshComponent.SetAnimInstanceClass` (`SkeletalMeshActor.SkeletalMeshComponent` (`self.BasebodyHeadMesh`)) _animinstanceclass)
          (`SkeletalMeshComponent.SetAnimInstanceClass` (`SkeletalMeshActor.SkeletalMeshComponent` (`self.ThumbnailMesh`)) _animinstanceclass)
          (`SkinnedMeshComponent.SetSkinnedAssetAndUpdate` (`SkeletalMeshActor.SkeletalMeshComponent` (`self.BasebodyBodyMesh`)) _bodymesh true)
          (`SkinnedMeshComponent.SetSkinnedAssetAndUpdate` (`SkeletalMeshActor.SkeletalMeshComponent` (`self.BasebodyHeadMesh`)) _headmesh true)
          (for _index (range (`PrimitiveComponent.GetNumMaterials` _skeletalmeshcomponent_2))
            (`PrimitiveComponent.SetMaterial` _skeletalmeshcomponent_2 _index "/Game/CharacterEditor/Base/Materials/MI_GreyBall.MI_GreyBall"))
          (for _index_2 (range (`PrimitiveComponent.GetNumMaterials` _skeletalmeshcomponent))
            (`PrimitiveComponent.SetMaterial` _skeletalmeshcomponent _index_2 "/Game/CharacterEditor/Base/Materials/MI_GreyBall.MI_GreyBall")))))))

(fn `UserConstructionScript`
  (`self.UpdateGenderVisuals`)
  (set `SceneCaptureComponent2D.TextureTarget` (`self.TextureTarget`) (`self.CaptureComponent2D`))
  (if (not (`self.EditSelectedCDAs`))
    (`BlueprintMapLibrary.Map_Clear` (`self.SelectedCDAs`))
    (bind _cda (`/Game/CharacterEditor/Base/Blueprints/Libraries/CharacterEditorFunctionLibrary.GetCDA_FromAssetRegistry` (`self.CDA_Class`) (`self.Anatomy`)))
    (for _array_element _cda
      (bind _asbp_cda_apparel (cast `/Game/CharacterEditor/Base/Blueprints/DataAssets/BP_CDA_Apparel` _array_element)
        (:`then`
          (bind _get (`/Game/CharacterEditor/Base/Blueprints/Libraries/CharacterEditorObjectMacros.TempValueByExec` (`/Game/CharacterEditor/Base/Blueprints/DataAssets/BP_CDA_Apparel.SkeletalMesh` _asbp_cda_apparel) (`/Game/CharacterEditor/Base/Blueprints/DataAssets/BP_CDA_Hairstyle.SkeletalMesh` (stale _asbp_cda_hairstyle)) :!label _label))
          (`BlueprintMapLibrary.Map_Add` (`self.SelectedCDAs`) (`KismetStringLibrary.Concat_StrStr` (`KismetSystemLibrary.GetDisplayName` _array_element) (`self.Suffix`)) _get))
        (:`CastFailed`
          (bind _asbp_cda_hairstyle (cast `/Game/CharacterEditor/Base/Blueprints/DataAssets/BP_CDA_Hairstyle` _array_element))
          (goto _label :!via `B `)))))
  (bind _values (`BlueprintMapLibrary.Map_Values` (`self.SelectedCDAs`)))
  (bind _returnvalue (`/Game/CharacterEditor/Base/Blueprints/Libraries/CharacterEditorObjectMacros.ValidatedGet` _values)
    (:`IsValid`
      (`SkinnedMeshComponent.SetSkinnedAssetAndUpdate` (`SkeletalMeshActor.SkeletalMeshComponent` (`self.ThumbnailMesh`)) _returnvalue true))))