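; Blueprint interface for the character customization system in the CharacterEditor base, defining how other code talks to a customizable character.
; It declares functions to add skeletal or static mesh components and to destroy a given component.
; Getters expose the character editor component, the character customization component and the customization profile.
; The functions are stubs with no logic, leaving behavior to implementing classes.
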(fn `AddSkeletalMeshComponent`
  (returns (ReturnValue :type "SkeletalMeshComponent Object Reference"))
  (return null))

(fn `AddStaticMeshComponent`
  (returns (ReturnValue :type "StaticMeshComponent Object Reference"))
  (return null))

(fn `DestroyComponent`
  (params (Component :type "ActorComponent Object Reference"))
  (returns (ReturnValue :type Boolean))
  (return false))

(fn `GetCharacterCustomizationComponent`
  (returns (ReturnValue :type "/Game/CharacterEditor/Base/Blueprints/Components/BP_CharacterCustomization Object Reference"))
  (return null))

(fn `GetCharacterEditorComponent`
  (returns (ReturnValue :type "/Game/CharacterEditor/Base/Blueprints/Components/BP_CharacterEditor Object Reference"))
  (return null))

(fn `GetCustomizationProfile`
  (returns (ReturnValue :type "/Game/CharacterEditor/Base/Structures/FCustomizationProfile_V4 Structure"))
  (return))